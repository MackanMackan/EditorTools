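; Scatters instances of a chosen static mesh over the ground in a rectangular area around the actor.
; The Construction Script fills an InstancedStaticMesh with NumberOfObjects world-space instances placed by GetRandomTransform.
; Each transform picks seeded random XY within SpawnAreaSize, traces vertically against SurfaceObjectTypes, and optionally aligns to the hit normal via RotateWithGround.
; BeginPlay only runs an empty loop.
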(event EventBeginPlay
  (for _index (range 0 (- (Variables|Default|GetNumberOfObjects) 1))
    _))

(event Collision|EventActorBeginOverlap
  (params (OtherActor :type Actor%20Object%20Reference)))

(event EventTick
  (params (DeltaSeconds :type Float%20%28single-precision%29)))

(fn ConstructionScript
  (Utilities|FlowControl|Sequence
    (:then_0
      (Components|StaticMesh|SetStaticMesh (Variables|Default|GetInstancedStaticMesh) (Variables|Default|GetActiveStaticMesh)))
    (:then_1
      (for _index (range 0 (- (Variables|Default|GetNumberOfObjects) 1))
        (Components|InstancedStaticMesh|AddInstance (Variables|Default|GetInstancedStaticMesh) (CallFunction|GetRandomTransform) true)))))

(fn GetRandomTransform
  (bind _returnvalue (Transformation|GetActorLocation))
  (bind _spawnareasize (Variables|Default|GetSpawnAreaSize))
  (bind _randomseed (Variables|Default|GetRandomSeed))
  (bind _returnvalue_2 (* (.x _spawnareasize) 25.0))
  (bind _returnvalue_3 (* (.y _spawnareasize) 25.0))
  (bind _returnvalue_4 (- (.y _returnvalue) _returnvalue_3))
  (bind _returnvalue_5 (+ (.y _returnvalue) _returnvalue_3))
  (bind _returnvalue_6 (- (.x _returnvalue) _returnvalue_2))
  (bind _returnvalue_7 (+ (.x _returnvalue) _returnvalue_2))
  (bind _returnvalue_8 (Math|Random|RandomFloatinRangefromStream _randomseed _returnvalue_6 _returnvalue_7))
  (bind _returnvalue_9 (Math|Random|RandomFloatinRangefromStream _randomseed _returnvalue_4 _returnvalue_5))
  (bind _returnvalue_10 (Math|Vector|MakeVector _returnvalue_8 _returnvalue_9 1e+04))
  (bind _outhit (Collision|LineTraceForObjects (Math|Vector|MakeVector (.x _returnvalue_10) (.y _returnvalue_10) (.z _returnvalue_10)) (Math|Vector|MakeVector (.x _returnvalue_10) (.y _returnvalue_10) (* (.z _returnvalue_10) -1.0)) (Variables|Default|GetSurfaceObjectTypes) false 0 "None"))
  (if (Variables|Default|GetRotateWithGround)
    (return (Math|Transform|MakeTransform (.location _outhit) (Math|Rotator|MakeRotfromZ (.normal _outhit))))
    (else
      (return (Math|Transform|MakeTransform (.location _outhit))))))